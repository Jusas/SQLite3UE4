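; BP_UnrealChair is a test Blueprint that exercises SQLite database queries on BeginPlay.
; It registers TestDatabase from a content-relative file if needed, then fills its own properties from the first "ikea" row in the Furniture table using raw SQL.
; A second query, built with query-builder nodes, fetches furniture under a price limit and prints each field's key and value.
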(event EventBeginPlay
  (bind _returnvalue (Class|SQLiteDatabase|IsDatabaseRegistered "TestDatabase"))
  (if _returnvalue
    (Development|PrintString "Second check - Database Registered!")
    (else
      (Class|SQLiteDatabase|RegisterDatabase "TestDatabase" "/Databases/TestDatabase.db" true)))
  (Class|SQLiteDatabase|GetDataIntoObject "TestDatabase" "SELECT * FROM Furniture WHERE Vendor = \"ikea\" LIMIT 1" self)
  (bind _returnvalue_2 (Class|SQLiteDatabase|GetDataBP (Utilities|Struct|MakeSQLiteDatabaseReference "TestDatabase" (Utilities|Array|MakeArray "Furniture")) (Utilities|Array|MakeArray "*") (Class|SQLiteBlueprintFunctionLibrary|QueryFinal (Class|SQLiteBlueprintFunctionLibrary|QueryEnd (Class|SQLiteBlueprintFunctionLibrary|QueryTerm (Class|SQLiteBlueprintFunctionLibrary|QueryStart) "Price" "<" "100"))) -1))
  (for _array_element (.ResultRows (Utilities|Struct|BreakSQLiteQueryResult _returnvalue_2))
    (for _array_element_2 (Utilities|Struct|BreakSQLiteQueryResultRow _array_element)
      (Development|PrintString (Utilities|String|Append (Class|KismetStringLibrary|RightPad (.Key (Utilities|Struct|BreakSQLiteKeyValuePair _array_element_2)) 1) (.Value (Utilities|Struct|BreakSQLiteKeyValuePair _array_element_2)))))))

(fn ConstructionScript)